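; Level exit zone that advances the game to the next level once the player enters it with all crystals gone.
; On actor overlap it filters for the player, then a pure const check confirms no BP_Crystal actors remain.
; The current level's position in the LevelNames array selects the next level to open by name.
; On the final level, completion does nothing.
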(event `self.ReceiveActorBeginOverlap`
  (params (OtherActor :type "Actor Object Reference"))
  (`/Game/Blueprints/CrystalCavernsMacroLib.IsPlayer` OtherActor
    (:`Is Player`
      (if (not (`self.Any Crystals Left`))
        (`self.Complete Level`)))))

(fn `Any Crystals Left`
  (returns (AnyCrystalsLeft :type Boolean))
  ;[1 0.474 0.474 1 12] Checked box for pure and const in order to ensure this function NEVER changes the state of anything
  (bind _outactors (`GameplayStatics.GetAllActorsOfClass` "/Game/Blueprints/Collectibles/BP_Crystal.BP_Crystal_C"))
  ;[1 0.4792 0.4792 1 12] Without it, functions can continue to use blocks that affect state and we may unknowingly be changing things as a result
  (return (> (`KismetArrayLibrary.Array_Length` _outactors) 0)))

(fn `Complete Level`
  (if (not (`self.Is Final Level`))
    (`self.Load Next Level`)))

(fn `Get Current Level Index`
  (returns (`Return Value` :type Integer))
  (bind _returnvalue (`GameplayStatics.GetCurrentLevelName` true))
  (return (`KismetArrayLibrary.Array_Find` (`self.Level Names`) (`KismetStringLibrary.Conv_StringToName` _returnvalue))))

(fn `Get Next Level Name`
  (returns (`Return Value` :type "Name (by ref)"))
  (return (`|GetArrayItem` (`self.Level Names`) (+ (`self.Get Current Level Index`) 1))))

(fn `Is Final Level`
  (returns (`Return Value` :type Boolean))
  (return (== (`KismetArrayLibrary.Array_LastIndex` (`self.Level Names`)) (`self.Get Current Level Index`))))

(fn `Load Next Level`
  (`GameplayStatics.OpenLevel` (`self.Get Next Level Name`)))

(fn `UserConstructionScript`)