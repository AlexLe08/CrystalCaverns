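; BP_Cannon is an obstacle cannon that repeatedly fires BP_Projectile actors, starting at BeginPlay.
; After a FireRate delay, it spawns a projectile at ProjectileSpawnPoint's location and rotation, scaled by ProjectileScale.
; The CannonFire timeline then animates the barrel along its relative Y axis, and its Cannon Fired output loops back to the delay for the next shot.
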(event `self.ReceiveBeginPlay`
  (`KismetSystemLibrary.Delay` (`self.Fire Rate`) :!label _label)
  (`self.Spawn projectile`)
  ;[1 1 1] Animated cannon barrel
  (bind (_direction _cannonbarrellocation) (`Timeline|CannonFire` :!via `PlayFromStart`)
    (:`Update`
      (`self.Move Cannon Barrel` _cannonbarrellocation))
    (:`Cannon Fired`
      (goto _label))))

(fn `Move Cannon Barrel`
  (params (`Cannon Barrel Y` :type "Float (double-precision)"))
  (`SceneComponent.K2_SetRelativeLocation` (`self.CannonBarrel`) (`KismetMathLibrary.MakeVector` 0.0 `Cannon Barrel Y`) false false))

(fn `Spawn projectile`
  (bind _projectilespawnpoint (`self.ProjectileSpawnPoint`))
  (`|SpawnActorFromClass` "/Game/Blueprints/Obstacles/BP_Projectile.BP_Projectile_C" (`KismetMathLibrary.MakeTransform` (`SceneComponent.K2_GetComponentLocation` _projectilespawnpoint) (`SceneComponent.K2_GetComponentRotation` _projectilespawnpoint) (`KismetMathLibrary.Conv_DoubleToVector` (`self.Projectile Scale`))) "Undefined" "OverrideRootScale" null null))

(fn `UserConstructionScript`)