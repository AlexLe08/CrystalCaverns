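; BP_Crystal is a collectible crystal that the player picks up by overlapping it.
; An IsPlayer macro filters the overlap to the player pawn, then the crystal stores its starting location, scale and light intensity.
; A timeline then lerps it toward the player's current position while shrinking it and dimming its point light, and destroys it when finished.
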(event `self.ReceiveActorBeginOverlap`
  (params (OtherActor :type "Actor Object Reference"))
  ;[1 1 1] Check if player overlaps crystal before collecting it; destroying it
  (`self.IsPlayer` OtherActor ; Difference between BP Functions and BP Macros is Macros can have multiple Execution pins
    (:`IsPlayer`
      ;;[1 1 1] Smooth movement of crystal to player
      (`self.StoreStartingValues`)
      (bind (_direction _move_progress _scale_progress _intensity_progress) (`Timeline|Collection Timeline`)
        (:`Update`
          ;;;[1 1 1 1 14] BP Functions can keep code tidy
          (`self.MoveToPlayer` _move_progress)
          (`self.ScaleCrystal` _scale_progress)
          (`self.AdjustLight` _intensity_progress))
        (:`Finished`
          (`self.K2_DestroyActor`))))))

(fn `AdjustLight`
  (params (Alpha :type "Float (double-precision)"))
  (`LightComponent.SetIntensity` (`self.Crystal_PointLight`) (`KismetMathLibrary.Lerp` (`self.StartIntensity`) 0.0 Alpha)))

(fn `MoveToPlayer`
  (params (Alpha :type "Float (double-precision)"))
  (`self.K2_SetActorLocation` (`KismetMathLibrary.VLerp` (`self.Start Location`) (`self.K2_GetActorLocation` (`GameplayStatics.GetPlayerPawn` 0)) Alpha)))

(fn `ScaleCrystal`
  (params (Alpha :type "Float (double-precision)"))
  (`self.SetActorScale3D` (`KismetMathLibrary.VLerp` (`self.StartScale`) (0.0 0.0 0.0) Alpha)))

(fn `StoreStartingValues`
  (set `self.Start Location` (`self.K2_GetActorLocation`))
  (set `self.StartScale` (`self.GetActorScale3D`))
  (set `self.StartIntensity` (`LightComponentBase.Intensity` (`self.Crystal_PointLight`))))

(fn `UserConstructionScript`)