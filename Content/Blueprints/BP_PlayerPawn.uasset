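; BP_PlayerPawn is the player pawn, moved by applying physics torque to its static mesh, with a camera fade-in on BeginPlay.
; The forward/backward and right/left axis inputs add mass-independent torque around Y and X, scaled by AccelerationMultiplier.
; When IsDead is set, both inputs instead share one branch that hides the mesh and stops its physics simulation for a "deathcam" mode.
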(event `self.ReceiveBeginPlay`
  ;[1 1 1] Camera fade in
  (`PlayerCameraManager.StartCameraFade` :`self` (`GameplayStatics.GetPlayerCameraManager` 0) :`FromAlpha` 1.0 :`Duration` 2.0))

(event `InputAxis|Move Forwards/Backwards`
  (params (AxisValue :type "Float (single-precision)"))
  (bind _staticmesh (`self.StaticMesh`))
  ;[1 1 1] Player Movement
  ;;[1 0.2185 0.2384] Check for death to enter "deathcam" mode
  (if (`self.isDead`)
    (`SceneComponent.SetVisibility` _staticmesh false false :!label _label)
    (`PrimitiveComponent.SetSimulatePhysics` _staticmesh false)
    (else
      (`PrimitiveComponent.AddTorqueInRadians` (`self.StaticMesh`) (`KismetMathLibrary.MakeVector` 0.0 (* AxisValue (`self.Acceleration Multiplier`))) "None" true))))

(event `InputAxis|Move Right/Left`
  (params (AxisValue :type "Float (single-precision)"))
  ;[1 1 1] Player Movement
  ;;[1 0.2185 0.2384] Check for death to enter "deathcam" mode
  (if (`self.isDead`)
    (goto _label)
    (else
      (`PrimitiveComponent.AddTorqueInRadians` (`self.StaticMesh`) (`KismetMathLibrary.MakeVector` (* AxisValue (`self.Acceleration Multiplier`))) "None" true))))

(fn `UserConstructionScript`)